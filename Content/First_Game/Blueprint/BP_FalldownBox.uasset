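; BP_FalldownBox is a spinning obstacle that ragdolls the player character when hit.
; On BeginPlay a fast looping timer calls Swing, which uses TurnObject to yaw the Cube by a fixed step, so rotation runs without Tick.
; A Cube hit by a BP_Character prints a message and calls that character's DoRagdoll.
; The overlap events are empty.
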(event `self.ReceiveBeginPlay`
  (`KismetSystemLibrary.K2_SetTimer` null "Swing" 0.01 true))

(event `self.ReceiveTick`
  (params (DeltaSeconds :type "Float (single-precision)")))

(event `self.Cube.OnComponentBeginOverlap`
  (params (OverlappedComponent :type "PrimitiveComponent Object Reference") (OtherActor :type "Actor Object Reference") (OtherComp :type "PrimitiveComponent Object Reference") (OtherBodyIndex :type Integer) (bFromSweep :type Boolean) (SweepResult :type "HitResult Structure (by ref)")))

(event `self.Cube.OnComponentHit`
  (params (HitComponent :type "PrimitiveComponent Object Reference") (OtherActor :type "Actor Object Reference") (OtherComp :type "PrimitiveComponent Object Reference") (NormalImpulse :type "Vector Structure") (Hit :type "HitResult Structure (by ref)"))
  (bind _asbp_character (cast `/Game/First_Game/Gamemode/BP_Character` OtherActor))
  (`KismetSystemLibrary.PrintString` "Oops!")
  (`/Game/First_Game/Gamemode/BP_Character.DoRagdoll` _asbp_character))

(fn `Swing`
  (`self.TurnObject` 0.01))

(fn `TurnObject`
  (params (Speed :type "Float (double-precision)"))
  (`SceneComponent.K2_AddWorldRotation` (`self.Cube`) (`KismetMathLibrary.MakeRotator` 0.0 0.0 (* Speed 500.0)) false false))

(fn `UserConstructionScript`)