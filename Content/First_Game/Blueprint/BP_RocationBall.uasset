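; BP_RocationBall is a hazard actor whose Sphere spins and moves up and down, ragdolling a BP_Character that hits it.
; A looping timer calls MoveBall and Turn to yaw the Sphere.
; Tick drives a timeline that sets the Sphere's relative Z, flipping IsRight on finish to alternate play and reverse.
; A hit on the Center component casts the other actor to BP_Character and calls DoRagdoll.
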(event `self.ReceiveBeginPlay`
  (`KismetSystemLibrary.K2_SetTimer` null "MoveBall" 0.01 true))

(event `self.ReceiveTick`
  (params (DeltaSeconds :type "Float (single-precision)"))
  (if (`self.IsRight`) :!label _label
    (bind (_direction `_새_트랙_0`) (`Timeline|타임라인_0` :`NewTime` 2.0 :!label _label_2)
      (:`Update`
        (`SceneComponent.K2_SetRelativeLocation` (`self.Sphere`) (`KismetMathLibrary.MakeVector` 0.0 0.0 (* `_새_트랙_0` 60.0)) false false))
      (:`Finished`
        (set `self.IsRight` (not (`self.IsRight`)))
        (goto _label)))
    (else
      (goto _label_2 :!via `Reverse`))))

(event `self.Center.OnComponentHit`
  (params (HitComponent :type "PrimitiveComponent Object Reference") (OtherActor :type "Actor Object Reference") (OtherComp :type "PrimitiveComponent Object Reference") (NormalImpulse :type "Vector Structure") (Hit :type "HitResult Structure (by ref)"))
  (bind _asbp_character (cast `/Game/First_Game/Gamemode/BP_Character` OtherActor))
  (`/Game/First_Game/Gamemode/BP_Character.DoRagdoll` _asbp_character))

(fn `MoveBall`
  (`self.Turn` 0.01))

(fn `Turn`
  (params (NewParam :type "Float (double-precision)"))
  (`SceneComponent.K2_AddLocalRotation` (`self.Sphere`) (`KismetMathLibrary.MakeRotator` 0.0 0.0 (* NewParam 100.0)) false false))

(fn `UserConstructionScript`)